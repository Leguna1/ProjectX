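; Ability component that gates three abilities behind individual cooldowns, ignoring a trigger while that ability is still cooling down.
; A successful trigger copies its duration from AbilityCooldowns into the ActiveCooldowns map and sets a shared looping 0.1-second timer.
; Each tick calls all three activation events, decrements and removes expired entries, and clears the timer once the map empties.
; It also stores an assigned array of cooldown widgets.
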(event Custom|TriggerAbility3
  ;[0.2033 1 0] Ability3
  (if (not (Utilities|Map|Contains (Variables|Default|GetActiveCooldowns) "Ability3"))
    (Utilities|Map|Add (Variables|Default|GetActiveCooldowns) "Ability3" (.Value (Utilities|Map|Find (Variables|Default|GetAbilityCooldowns) "Ability3")))
    (CallFunction|CooldownTimer)
    (Development|PrintString "Ability 3: Triggered..")))

(event Custom|TriggerAbility1
  ;[0.599 0.0231 0] Ability 1
  (if (not (Utilities|Map|Contains (Variables|Default|GetActiveCooldowns) "Ability1"))
    (Utilities|Map|Add (Variables|Default|GetActiveCooldowns) "Ability1" (.Value (Utilities|Map|Find (Variables|Default|GetAbilityCooldowns) "Ability1")))
    (CallFunction|CooldownTimer)
    (Development|PrintString "Ability 1: Triggered..")))

(event Custom|TriggerAbility2
  ;[0 0.01884 1] Ability 2
  (if (not (Utilities|Map|Contains (Variables|Default|GetActiveCooldowns) "Ability2"))
    (Utilities|Map|Add (Variables|Default|GetActiveCooldowns) "Ability2" (.Value (Utilities|Map|Find (Variables|Default|GetAbilityCooldowns) "Ability2")))
    (CallFunction|CooldownTimer)
    (Development|PrintString "Ability 2: Triggered..")))

(event Custom|CooldownTick
  ;[0.3177 0.3177 0.3177] Cooldown Timer
  (CallFunction|CallonEvents)
  (bind _keys (Utilities|Map|Keys (Variables|Default|GetActiveCooldowns)))
  (for _array_element _keys
    (if (> (.Value (Utilities|Map|Find (Variables|Default|GetActiveCooldowns) _array_element)) 0.0)
      (Utilities|Map|Add (Variables|Default|GetActiveCooldowns) _array_element (- (.Value (Utilities|Map|Find (Variables|Default|GetActiveCooldowns) _array_element)) 0.1))
      (bind _output_get (Variables|Default|SetActiveCooldowns (Variables|Default|GetActiveCooldowns)))
      (if (<= (.Value (Utilities|Map|Find _output_get _array_element)) 0.0)
        (bind _returnvalue (Utilities|Map|Remove _output_get _array_element))
        (Development|PrintString (Utilities|String|ToString(Boolean) _returnvalue)))))
  (if (<= (Utilities|Map|Length (Variables|Default|GetActiveCooldowns)) 0)
    (Utilities|Time|ClearandInvalidateTimerbyHandle (Variables|Default|GetCooldownTimerHandle))))

(event Custom|CooldownTimer
  ;[0.3177 0.3177 0.3177] Cooldown Timer
  (if (> (Utilities|Map|Length (Variables|Default|GetActiveCooldowns)) 0)
    (bind _returnvalue (Utilities|Time|SetTimerbyEvent (delegate Custom|CooldownTick) 0.1 true))
    (Variables|Default|SetCooldownTimerHandle _returnvalue)))

(event Custom|AssignCooldownWidgets
  (params (Widgets :type String) (CooldownWidgetArray :type Array%20of%20WB%20Ability%20Cooldown%20Object%20References))
  (Variables|Default|SetCooldown%20Widget%20Array CooldownWidgetArray))

(event Custom|CallOnEvents
  (Default|CallOnAbilityOneActivation)
  (Default|CallOnAbilityTwoActivation)
  (Default|CallOnAbilityThreeActivation))

(event EventBeginPlay)
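; BP_WeaponBase is a weapon base Blueprint with an early hit test for attacking a given target.
; Its Active event runs a debug-drawn line trace for Pawns between Start and End, ignoring the Owner.
; A hit on the passed Target that implements BPI_Damageable only prints a placeholder message, with no damage applied.
; Tick and the construction script are empty.
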(event Custom|Active
  (params (Owner :type Character%20Object%20Reference) (Target :type Character%20Object%20Reference))
  (bind _outhit (Collision|LineTraceForObjects (Variables|Default|GetStart) (Variables|Default|GetEnd) (Utilities|Array|MakeArray "ObjectTypeQuery3") false (Utilities|Array|MakeArray Owner) "ForDuration" true "(R=1.000000,G=0.000000,B=0.000000,A=1.000000)" "(R=0.000000,G=1.000000,B=0.000000,A=1.000000)" 1.0))
  (if (and (Utilities|DoesObjectImplementInterface (.HitActor (Collision|BreakHitResult _outhit)) "/Game/Developers/KalE/Systems/DamageSystem/BPI_Damageable.BPI_Damageable_C") (== (.HitActor (Collision|BreakHitResult _outhit)) Target))
    (Development|PrintString "Hello")))

(event EventTick
  (params (DeltaSeconds :type Float%20%28single-precision%29)))

(fn ConstructionScript)
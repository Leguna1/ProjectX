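; Animation notify that plays surface-dependent footstep sounds and reports each step as noise from the owner's Instigator pawn.
; On notify, it traces down from the owning actor on the Visibility channel and, on a hit, calls PawnMakeNoise at the actor's location.
; The hit's surface type selects a grass, sand, wood, stone or water sound, played at world origin rather than the actor's location.
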(fn ReceivedNotify
  (params (MeshComp :type Skeletal%20Mesh%20Component%20Object%20Reference) (Animation :type Anim%20Sequence%20Base%20Object%20Reference) (EventReference :type Anim%20Notify%20Event%20Reference%20Structure%20%28by%20ref%29))
  (bind _returnvalue (Components|GetOwner MeshComp))
  (bind _returnvalue_2 (Transformation|GetActorLocation _returnvalue))
  (bind _instigator (Variables|/Script/Engine.Actor|GetInstigator _returnvalue))
  (bind (_outhit _returnvalue_3) (Collision|LineTraceByChannel _returnvalue_2 (+ _returnvalue_2 (* (Transformation|GetActorUpVector _returnvalue) -2e+02)) "TraceTypeQuery1" false 0 "None"))
  (if _returnvalue_3
    (Class|Pawn|PawnMakeNoise _instigator 1.0 _returnvalue_2 true _instigator)
    (switch Utilities|FlowControl|Switch|SwitchonEPhysicalSurface (Collision|GetSurfaceType _outhit)
      (:SurfaceType1
        (Audio|PlaySoundatLocation "/Game/Sounds/S_Grass_Mono_Without_Hitting_Boot_4_Cue.S_Grass_Mono_Without_Hitting_Boot_4_Cue" "0, 0, 0" "0, 0, 0" 1.0 1.0 0.0 0 0 0 0))
      (:SurfaceType2
        (Audio|PlaySoundatLocation "/Game/Sounds/S_Sand_Mono_1_Cue.S_Sand_Mono_1_Cue" "0, 0, 0" "0, 0, 0" 1.0 1.0 0.0 0 0 0 0))
      (:SurfaceType3
        (Audio|PlaySoundatLocation "/Game/SmallSoundKit/SSKWav/FootstepsWav/S_Wood_Mono_2.S_Wood_Mono_2" "0, 0, 0" "0, 0, 0" 1.0 1.0 0.0 0 0 0 0))
      (:SurfaceType4
        (Audio|PlaySoundatLocation "/Game/SmallSoundKit/SSKWav/FootstepsWav/S_Concrete_Mono_2.S_Concrete_Mono_2" "0, 0, 0" "0, 0, 0" 1.0 1.0 0.0 0 0 0 0))
      (:SurfaceType5
        (Audio|PlaySoundatLocation "/Engine/EditorSounds/GamePreview/PossessPlayer_Cue.PossessPlayer_Cue" "0, 0, 0" "0, 0, 0" 1.0 1.0 0.0 0 0 0 0))))
  (return false))